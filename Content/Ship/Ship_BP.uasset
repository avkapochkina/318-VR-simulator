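; Player ship pawn prototype with keyboard axis controls and disconnected Arduino serial control.
; Forward_Back accumulates force pushed along the flattened forward vector at the collision's center of mass; Right_Left accumulates controller yaw, though a note marks keyboard movement non-working.
; Unwired serial logic would send a position-sign code, read wheel and arm speeds every few passes, and rotate and offset the ship mesh.
; Tick and construction script are empty.
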(event `self.ReceiveTick`
  (params (DeltaSeconds :type "Float (single-precision)"))
  ;[1 1 1] Sending request and receiving data
)

(event `InputAxis|Forward_Back`
  (params (AxisValue :type "Float (single-precision)"))
  (bind (_returnvalue_x _returnvalue_y) (`KismetMathLibrary.BreakVector` (`self.GetActorForwardVector`)))
  ;[1 1 1] Keyboard movement (off for now) (doesn't work)
  (bind _output_get (set `self.CoefForce` (* AxisValue 10000.0)))
  (bind _output_get_2 (set `self.Force` (+ (`self.Force`) _output_get)))
  (`PrimitiveComponent.AddForceAtLocation` (`self.CollisionComponent`) (* (`KismetMathLibrary.MakeVector` _returnvalue_x _returnvalue_y) _output_get_2) (`PrimitiveComponent.GetCenterOfMass` (`self.CollisionComponent`) "None") "None")
  (`KismetSystemLibrary.PrintString` (`KismetStringLibrary.Conv_DoubleToString` _output_get_2)))

(event `InputAxis|Right_Left`
  (params (AxisValue :type "Float (single-precision)"))
  ;[1 1 1] Keyboard movement (off for now) (doesn't work)
  (bind _output_get (set `self.Yaw` (+ (* AxisValue 0.005) (`self.Yaw`))))
  (`self.AddControllerYawInput` _output_get))

(fn `UserConstructionScript`)