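; Test ship pawn driven by keyboard, with flow and wind offsets added to its motion.
; Forward input accumulates velocity into a forward force at the center of mass; steering accumulates controller yaw, with key releases resetting each.
; Releasing M swaps all widgets for the flow/wind UI.
; Arduino serial control, reading wheel and arm speeds and returning a position code, is disconnected from BeginPlay, Tick and EndPlay, so never runs.
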(event `Key|M`
  (params (Key :type "Key Structure"))
  ;[1 1 1] Widjets
  (:`Released`
    (`self.show_ui_vidjet` "/Game/UI/UI_Flow+Wind.UI_Flow+Wind_C")))

(event `InputAxis|Forward_Back`
  (params (AxisValue :type "Float (single-precision)"))
  (bind (_returnvalue_x _returnvalue_y) (`KismetMathLibrary.BreakVector` (`self.GetActorForwardVector`)))
  ;[1 1 1] Keyboard movement (on for now)
  (bind _output_get (set `self.Velocity` (+ (* AxisValue (`self.Acceleration`)) (`self.Velocity`))))
  (bind _output_get_2 (set `self.YSpeed` (+ _output_get (`self.YFlow`) (`self.YWind`))))
  (`PrimitiveComponent.AddForceAtLocation` (`self.CollisionComponent`) (* (`KismetMathLibrary.MakeVector` _returnvalue_x _returnvalue_y) _output_get_2) (`PrimitiveComponent.GetCenterOfMass` (`self.CollisionComponent`) "None") "None"))

(event `InputAxis|Right_Left`
  (params (AxisValue :type "Float (single-precision)"))
  (bind _returnvalue (+ (* AxisValue 0.005) (`self.Yaw`) (`self.XFlow`) (`self.XWind`)))
  ;[1 1 1] Keyboard movement (on for now)
  (if (> 1.0 _returnvalue)
    (bind _output_get (set `self.Yaw` _returnvalue))
    (`self.AddControllerYawInput` _output_get)))

(event `Key|A`
  (params (Key :type "Key Structure"))
  ;[1 1 1] Keyboard movement (on for now)
  (:`Released`
    (set `self.Yaw` 0.0)))

(event `Key|D`
  (params (Key :type "Key Structure"))
  ;[1 1 1] Keyboard movement (on for now)
  (:`Released`
    (set `self.Yaw` 0.0)))

(event `Key|SpaceBar`
  (params (Key :type "Key Structure"))
  ;[1 1 1] Keyboard movement (on for now)
  (:`Released`
    (set `self.Velocity` 0.0)))

(event `self.ReceiveTick`
  (params (DeltaSeconds :type "Float (single-precision)"))
  ;[1 1 1] Sending request and receiving data
)

(event `self.ReceiveBeginPlay`)

(event `self.ReceiveEndPlay`
  (params (EndPlayReason :type "EEndPlayReason Enum" :default "Destroyed"))
  ;[1 1 1] Close Port
)

(fn `show_ui_vidjet`
  (params (Class :type "UserWidget Class Reference"))
  (`WidgetLayoutLibrary.RemoveAllWidgets`)
  (bind _returnvalue (`|CreateWidget` Class (`GameplayStatics.GetPlayerController` 0)))
  (`UserWidget.AddToViewport` _returnvalue 0))

(fn `UserConstructionScript`)