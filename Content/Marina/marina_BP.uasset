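; Marina obstacle actor that penalizes the test ship for hitting it by sending it back to a fixed reset position.
; BeginPlay creates hidden warning and timer widgets and caches the first Test_Ship_BP in the level.
; On a ship hit, a flag blocks re-triggering while the widgets show, a sound plays and chained delays count Time down from five.
; The ship's location, rotation, velocity and yaw are then reset and the widgets hidden.
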(event `self.ReceiveBeginPlay`
  (bind _returnvalue (`|CreateWidget` "/Game/UI/UI_Warning.UI_Warning_C"))
  (bind _output_get (set `self.warrning_var` _returnvalue))
  (`UserWidget.AddToViewport` _output_get 0)
  (`Widget.SetVisibility` (`self.warrning_var`) "Hidden")
  (bind _outactors (`GameplayStatics.GetAllActorsOfClass` "/Game/Ship/test_Ship_BP.test_Ship_BP_C"))
  (bind _astest_ship_bp (cast `/Game/Ship/test_Ship_BP` (`|GetArrayItem` _outactors)))
  (set `self.test_ship_var` _astest_ship_bp)
  (bind _returnvalue_2 (`|CreateWidget` "/Game/UI/UI_timer.UI_timer_C"))
  (bind _output_get_2 (set `self.timer_var` _returnvalue_2))
  (`UserWidget.AddToViewport` _output_get_2 0)
  (`Widget.SetVisibility` (`self.timer_var`) "Hidden")
  (set `self.collision_flag` true))

(event `self.ReceiveHit`
  (params (MyComp :type "PrimitiveComponent Object Reference") (Other :type "Actor Object Reference") (OtherComp :type "PrimitiveComponent Object Reference") (bSelfMoved :type Boolean) (HitLocation :type "Vector Structure") (HitNormal :type "Vector Structure") (NormalImpulse :type "Vector Structure") (Hit :type "HitResult Structure (by ref)"))
  (cast `/Game/Ship/test_Ship_BP` Other)
  (if (`self.collision_flag`)
    (set `self.collision_flag` false)
    (`Widget.SetVisibility` (`self.warrning_var`) "Visible")
    (`Widget.SetVisibility` (`self.timer_var`) "Visible")
    (`GameplayStatics.PlaySound2D` "/Game/Audio/Collision_sound.Collision_sound" 1.0 1.0 0.0 null null)
    (set `self.time` 5)
    (`KismetSystemLibrary.Delay` 1.0)
    (set `self.time` 4)
    (`KismetSystemLibrary.Delay` 1.0)
    (set `self.time` 3)
    (`KismetSystemLibrary.Delay` 1.0)
    (set `self.time` 2)
    (`KismetSystemLibrary.Delay` 1.0)
    (set `self.time` 1)
    (`KismetSystemLibrary.Delay` 1.0)
    (set `self.time` 0)
    (`self.K2_SetActorLocation` (`self.test_ship_var`) (-8220.0 6560.0 -6210.0) false false)
    (set `self.collision_flag` true)
    (set `/Game/Ship/test_Ship_BP.Velocity` 0.0 (`self.test_ship_var`))
    (set `/Game/Ship/test_Ship_BP.Yaw` 0.0 (`self.test_ship_var`))
    (`self.K2_SetActorRotation` :`self` (`self.test_ship_var`))
    (`Widget.SetVisibility` (`self.warrning_var`) "Hidden")
    (`Widget.SetVisibility` (`self.timer_var`) "Hidden")))

(fn `UserConstructionScript`)